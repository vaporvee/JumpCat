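; Game instance that carries level progression and run totals (coins, gems, speedrun counter) across levels.
; Steps through an array of levels by index, opening the next one on NextLevel.
; ShowLevelScreening shows a level finish menu, or on the last level a game finish menu, flags the game as played through and resets progress.
; Coin and gem pickups add to totals and refresh the third-person character's HUD.
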(event `self.ReceiveInit`
  (set `self.Length` (- (`KismetArrayLibrary.Array_Length` (`self.Levels`)) 1)))

(event `/Game/Blueprints/LevelManager/LevelInterface.NextLevel`
  (bind _index (`self.Index`))
  (set `self.Index` (+ (`self.Index`) 1))
  (if (<= _index (`self.Length`))
    (`GameplayStatics.OpenLevelBySoftObjectPtr` (`|GetArrayItem` (`self.Levels`) _index))))

(event `/Game/Blueprints/LevelManager/LevelInterface.ShowLevelScreening`
  ;[1 1 1] Checkt ob das game durchgespielt wurde
  (if (<= (+ (`self.Index`) 1) (`self.Length`))
    (bind _returnvalue (`|CreateWidget` "/Game/Blueprints/Widgets/LevelFinishMenu.LevelFinishMenu_C"))
    (`UserWidget.AddToViewport` _returnvalue 0)
    (else
      (bind _returnvalue_2 (`|CreateWidget` "/Game/Blueprints/Widgets/GameFinishMenu.GameFinishMenu_C"))
      (`UserWidget.AddToViewport` _returnvalue_2 0)
      (set `self.PlayedThrough` true)
      ;[1 1 1] Reset
      (set `self.Index` 0)
      (set `self.Coins` 0)
      (set `self.Gems` 0)
      (set `self.SpeedrunCounter` 0.0))))

(event `/Game/Blueprints/LevelManager/LevelInterface.AddCoin`
  (params (Amount :type Integer))
  (set `self.Coins` (+ (`self.Coins`) Amount))
  (bind _asbp_third_person_character (cast `/Game/ThirdPerson/Blueprints/BP_ThirdPersonCharacter` (`GameplayStatics.GetPlayerCharacter` 0) :!label _label))
  (`/Game/Blueprints/Widgets/HUD.Update` (`/Game/ThirdPerson/Blueprints/BP_ThirdPersonCharacter.HUD` _asbp_third_person_character)))

(event `/Game/Blueprints/LevelManager/LevelInterface.AddGem`
  (params (Amount :type Integer))
  (set `self.Gems` (+ (`self.Gems`) Amount))
  (goto _label))