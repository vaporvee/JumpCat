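; LevelGoal is the level's end trophy, which closes out the level when its Overlap event fires.
; Overlap plays a backwards CircleTransition widget, flags the trophy as taken, pauses the third-person character, disables its input and hides the mesh.
; TransitionFinished then checks that flag, asks the game instance to show the level screening message, and clears the flag.
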(event `self.Overlap`
  (bind _returnvalue (`|CreateWidget` "/Game/Blueprints/Widgets/CircleTransition.CircleTransition_C" null true))
  (`UserWidget.AddToViewport` _returnvalue 0)
  (set `self.TrophyTaken` true)
  (bind _asbp_third_person_character (cast `/Game/ThirdPerson/Blueprints/BP_ThirdPersonCharacter` (`GameplayStatics.GetPlayerCharacter` 0)))
  (set `/Game/ThirdPerson/Blueprints/BP_ThirdPersonCharacter.Paused` true _asbp_third_person_character)
  (`self.DisableInput` _asbp_third_person_character (`GameplayStatics.GetPlayerController` 0))
  (`SceneComponent.SetVisibility` (`self.StaticMesh`) false false))

(event `/Game/Blueprints/LevelManager/LevelInterface.TransitionFinished`
  (if (`self.TrophyTaken`)
    (message `/Game/Blueprints/LevelManager/LevelInterface.ShowLevelScreening` (`GameplayStatics.GetGameInstance`))
    (set `self.TrophyTaken` false)))

(fn `UserConstructionScript`
  (`parent.UserConstructionScript`))