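; Game instance that manages progression through an ordered list of levels and shows the end-of-level screens.
; Init caches the last index of the Levels array, and NextLevel increments the current index and opens that level by object reference if within range.
; ShowLevelScreening adds a level-finish menu while levels remain, otherwise a game-finish menu and resets the index to the first level.
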(event `self.ReceiveInit`
  (set `self.Length` (- (`KismetArrayLibrary.Array_Length` (`self.Levels`)) 1)))

(event `/Game/Blueprints/LevelManage/LevelInterface.NextLevel`
  (bind _index (`self.Index`))
  (set `self.Index` (+ (`self.Index`) 1))
  (if (<= _index (`self.Length`))
    (`GameplayStatics.OpenLevelBySoftObjectPtr` (`|GetArrayItem` (`self.Levels`) _index))))

(event `/Game/Blueprints/LevelManage/LevelInterface.ShowLevelScreening`
  ;[1 1 1] Checkt ob das game durchgespielt wurde
  (if (<= (+ (`self.Index`) 1) (`self.Length`))
    (bind _returnvalue (`|CreateWidget` "/Game/Blueprints/Widgets/LevelFinishMenu.LevelFinishMenu_C"))
    (`UserWidget.AddToViewport` _returnvalue 0)
    (else
      (bind _returnvalue_2 (`|CreateWidget` "/Game/Blueprints/Widgets/GameFinishMenu.GameFinishMenu_C"))
      (`UserWidget.AddToViewport` _returnvalue_2 0)
      ;[1 1 1] Reset
      (set `self.Index` 0))))