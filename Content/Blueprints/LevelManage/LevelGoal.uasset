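; LevelGoal is the level's finish trophy, which spins every tick until the player collects it.
; When the player character overlaps its sphere, it starts a backwards circle transition widget, flags the trophy as taken, pauses the character, disables input and hides the trophy.
; Its TransitionFinished event then has the game instance show the level screening message and clears the flag.
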(event `self.ReceiveTick`
  (params (DeltaSeconds :type "Float (single-precision)"))
  ;[0 1 0.4721] Drehungs Animation
  (`SceneComponent.K2_AddRelativeRotation` (`self.Trophy`) (struct :`Yaw` 0.7) false false))

(event `self.Sphere.OnComponentBeginOverlap`
  (params (OverlappedComponent :type "PrimitiveComponent Object Reference") (OtherActor :type "Actor Object Reference") (OtherComp :type "PrimitiveComponent Object Reference") (OtherBodyIndex :type Integer) (bFromSweep :type Boolean) (SweepResult :type "HitResult Structure (by ref)"))
  (if (== (`GameplayStatics.GetPlayerCharacter` 0) OtherActor)
    (bind _returnvalue (`|CreateWidget` "/Game/Blueprints/Widgets/CircleTransition.CircleTransition_C" null true))
    (`UserWidget.AddToViewport` _returnvalue 0)
    (set `self.TrophyTaken` true)
    (bind _asbp_third_person_character (cast `/Game/ThirdPerson/Blueprints/BP_ThirdPersonCharacter` OtherActor))
    (set `/Game/ThirdPerson/Blueprints/BP_ThirdPersonCharacter.Paused` true _asbp_third_person_character)
    (`self.DisableInput` _asbp_third_person_character (`GameplayStatics.GetPlayerController` 0))
    (`SceneComponent.SetVisibility` (`self.Trophy`) false false)))

(event `/Game/Blueprints/LevelManage/LevelInterface.TransitionFinished`
  (if (`self.TrophyTaken`)
    (message `/Game/Blueprints/LevelManage/LevelInterface.ShowLevelScreening` (`GameplayStatics.GetGameInstance`))
    (set `self.TrophyTaken` false)))

(fn `UserConstructionScript`)